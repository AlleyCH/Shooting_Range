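; Range_Target_BP is a range target actor that slides back and forth continuously along the Y axis.
; BeginPlay stores the spawn position as Start and builds End from the same X and Z with a hardcoded Y.
; Two timelines chain in an endless loop: Move plays forward, then MoveBack plays in reverse, each lerping the location without sweep.
; Positions are read in world space but applied as relative location.
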(event EventBeginPlay
  (bind _returnvalue (Transformation|GetActorLocation))
  (Variables|Default|SetStart (Math|Vector|MakeVector (.x _returnvalue) (.y _returnvalue) (.z _returnvalue)))
  (Variables|Default|SetEnd (Math|Vector|MakeVector (.x _returnvalue) -1.73e+03 (.z _returnvalue)))
  (bind _move (Timeline|Move PlayFromStart)
    (:Update
      (Transformation|SetActorRelativeLocation (Math|Vector|Lerp(Vector) (Variables|Default|GetStart) (Variables|Default|GetEnd) _move)))
    (:Finished
      (bind _move_2 (Timeline|move%20back ReverseFromEnd)
        (:Update
          (Transformation|SetActorRelativeLocation (Math|Vector|Lerp(Vector) (Variables|Default|GetStart) (Variables|Default|GetEnd) _move_2)))
        (:Finished
          (Timeline|Move PlayFromStart))))))

(fn ConstructionScript)